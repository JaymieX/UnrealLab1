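; BP_RevolvingDoor is a door actor that rotates its mesh open when something overlaps its box collider and back when the overlap ends.
; A timeline plays forward on begin overlap and reverses on end overlap, driving the mesh's relative rotation from a vector track.
; Only yaw is offset by the rotation cached at BeginPlay, while roll and pitch come straight from the track.
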(event `self.ReceiveBeginPlay`
  (set `self.DoorInitRot` (`SceneComponent.RelativeRotation` (`self.DoorStaticMesh`))))

(event `self.BoxCollider.OnComponentBeginOverlap`
  (params (OverlappedComponent :type "PrimitiveComponent Object Reference") (OtherActor :type "Actor Object Reference") (OtherComp :type "PrimitiveComponent Object Reference") (OtherBodyIndex :type Integer) (bFromSweep :type Boolean) (SweepResult :type "HitResult Structure (by ref)"))
  (bind (_direction _door_rotation) (`Timeline|Door Time Line` :!label _label)
    (:`Update`
      (`SceneComponent.K2_SetRelativeRotation` (`self.DoorStaticMesh`) (`KismetMathLibrary.MakeRotator` (.x _door_rotation) (.y _door_rotation) (+ (.z _door_rotation) (.yaw (`self.DoorInitRot`)))) false false))))

(event `self.BoxCollider.OnComponentEndOverlap`
  (params (OverlappedComponent :type "PrimitiveComponent Object Reference") (OtherActor :type "Actor Object Reference") (OtherComp :type "PrimitiveComponent Object Reference") (OtherBodyIndex :type Integer))
  (goto _label :!via `Reverse`))

(fn `UserConstructionScript`)